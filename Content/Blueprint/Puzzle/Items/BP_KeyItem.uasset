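; BP_KeyItem is a puzzle key item that an interactor picks up from the world.
; GetItem runs the parent logic, passes the item's RowName from Collet to the interactor's AddItemMessage, then destroys the actor.
; The event graph holds only disabled default events, so the Blueprint's own behavior lives in these two functions.
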(fn `Collet`
  (params (Interactor :type "Actor Object Reference"))
  (returns (RowName :type Name))
  (return (`self.RowName`)))

(fn `GetItem`
  (params (Interactor :type "Actor Object Reference"))
  (`parent.GetItem` Interactor)
  (bind _rowname (`self.Collet` self null))
  (message `/Game/Blueprint/Interfacetable/BPI_InventoryInterface.AddItem` Interactor _rowname)
  (`self.K2_DestroyActor`))

(fn `UserConstructionScript`
  (`parent.UserConstructionScript`))
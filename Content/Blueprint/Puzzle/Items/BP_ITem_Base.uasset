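; BP_ITem_Base is a base Blueprint for interactable puzzle items, identified by a row name in DT_ItemData.
; On BeginPlay it sets its mesh and scale from that row, then after a short delay attaches itself to any overlapping BP_Door_Base mesh, keeping world transform, and sets its sphere to query-only.
; Interact calls GetItem, which is empty here, while Collet returns the row name.
; An unconnected line trace would snap the item to the ground.
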(event `self.ReceiveBeginPlay`
  (`self.ItemInit`)
  (`KismetSystemLibrary.Delay` 0.2)
  (`self.AttachActor`)
  (`PrimitiveComponent.SetCollisionEnabled` (`self.Sphere`) "QueryOnly"))

(event `/Game/Blueprint/Interfacetable/BPI_Interactable.Interact`
  (params (Interactor :type "Actor Object Reference"))
  (`self.GetItem` Interactor))

(fn `AttachActor`
  (for _array_element (`PrimitiveComponent.GetOverlappingActors` (`self.Sphere`) "/Game/Blueprint/Puzzle/Door/BP_Door_Base.BP_Door_Base_C")
    (bind _asbp_door_base (cast `/Game/Blueprint/Puzzle/Door/BP_Door_Base` (`ActorComponent.GetOwner` (`Actor.RootComponent` _array_element))))
    (bind _output_get (set `self.As BP Door Base` _asbp_door_base))
    (`self.K2_AttachToComponent` self (`/Game/Blueprint/Puzzle/Door/BP_Door_Base.StaticMesh` _output_get) "None" "KeepWorld" "KeepWorld" "KeepWorld" false)))

(fn `Collet`
  (params (Interactor :type "Actor Object Reference"))
  (returns (RowName :type Name))
  (return (`self.RowName`)))

(fn `GetItem`
  (params (Interactor :type "Actor Object Reference")))

(fn `getRowname`
  (returns (NewParam :type Name))
  (return (`self.RowName`)))

(fn `ItemInit`
  (bind _returnvalue (`|GetDataTableRow` "/Game/Blueprint/Datas/DataTable/DT_ItemData.DT_ItemData" (`self.RowName`))
    (:`then`
      (bind _output_get (set `self.Out Row` _returnvalue))
      (bind (_item_name _description _icon _3dmesh _type _scale) (break `/Game/Blueprint/Datas/Struct/ST_ItemData` _output_get))
      (`StaticMeshComponent.SetStaticMesh` (`self.StaticMesh`) _3dmesh)
      (`SceneComponent.SetWorldScale3D` (`self.StaticMesh`) _scale))))

(fn `UserConstructionScript`)
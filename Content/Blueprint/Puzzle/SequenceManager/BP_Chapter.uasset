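; BP_Chapter is a puzzle chapter in the sequence manager system that runs an ordered list of objectives one at a time.
; StartChapter resets the index and activates the first objective.
; Each OnObjectiveComplete call advances the index and activates the next objective, or notifies the sequence manager that the chapter is complete once the list runs out.
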(fn `OnObjectiveComplete`
  (set `self.CurrentObjectiveIndex` (+ (`self.CurrentObjectiveIndex`) 1))
  (if (>= (`self.CurrentObjectiveIndex`) (`KismetArrayLibrary.Array_Length` (`self.ObjectiveList`)))
    (`/Game/Blueprint/Puzzle/SequenceManager/BP_SequenceManager.OnChapterComplete` (`self.SequenceManagerRef`))
    (else
      (`/Game/Blueprint/Puzzle/SequenceManager/BP_Objective.Activate` (`|GetArrayItem` (`self.ObjectiveList`) (`self.CurrentObjectiveIndex`))))))

(fn `StartChapter`
  (bind _output_get (set `self.CurrentObjectiveIndex` 0))
  (`/Game/Blueprint/Puzzle/SequenceManager/BP_Objective.Activate` (`|GetArrayItem` (`self.ObjectiveList`) _output_get)))

(fn `UserConstructionScript`)
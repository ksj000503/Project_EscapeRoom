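; BP_Objective is a puzzle sequence objective that tracks completion of a list of interactables and reports to its chapter.
; At BeginPlay it takes the required total from the length of the interactable list.
; Once activated, each completion report increments a counter.
; When the counter equals the total, it notifies the referenced chapter that the objective is complete, while reports received before activation are ignored.
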(event `self.ReceiveBeginPlay`
  (set `self.TotalCount` (`KismetArrayLibrary.Array_Length` (`self.InteractableList`))))

(fn `Activate`
  (set `self.bIsActive` true))

(fn `ReportComplete`
  (if (`self.bIsActive`)
    (bind _result (`/Engine/EditorBlueprintResources/StandardMacros.IncrementInt` (`self.CompletedCount`))
      (:`  `
        (set `self.CompletedCount` _result)
        (if (== (`self.TotalCount`) (`self.CompletedCount`))
          (`/Game/Blueprint/Puzzle/SequenceManager/BP_Chapter.OnObjectiveComplete` (`self.ChapterRef`)))))))

(fn `UserConstructionScript`)
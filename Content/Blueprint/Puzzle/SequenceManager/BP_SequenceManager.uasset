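; BP_SequenceManager runs the puzzle chapters in order, one after another.
; It starts the first entry of ChapterList on BeginPlay.
; OnChapterComplete advances CurrentChapterIndex and starts the next chapter, or prints a game-over string once the list is exhausted.
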(event `self.ReceiveBeginPlay`
  (`/Game/Blueprint/Puzzle/SequenceManager/BP_Chapter.StartChapter` (`|GetArrayItem` (`self.ChapterList`))))

(fn `OnChapterComplete`
  (set `self.CurrentChapterIndex` (+ (`self.CurrentChapterIndex`) 1))
  (if (>= (`self.CurrentChapterIndex`) (`KismetArrayLibrary.Array_Length` (`self.ChapterList`)))
    (`KismetSystemLibrary.PrintString` "Gmae Over")
    (else
      (`/Game/Blueprint/Puzzle/SequenceManager/BP_Chapter.StartChapter` (`|GetArrayItem` (`self.ChapterList`) (`self.CurrentChapterIndex`))))))

(fn `UserConstructionScript`)
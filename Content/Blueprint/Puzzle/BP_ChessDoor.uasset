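; BP_ChessDoor is a puzzle door that swings open and closed.
; The construction script caches the actor's starting rotation as the closed pose.
; OpenDoor plays a Timeline that lerps the root component's relative rotation 90 degrees in yaw from that pose, printing a debug string on each update.
; Closed reverses the same Timeline, and both events update the IsOpend flag.
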(event `OpenDoor`
  (bind (_actorrotation_roll _actorrotation_pitch _actorrotation_yaw) (`KismetMathLibrary.BreakRotator` (`self.ActorRotation`)))
  (set `self.bIsOpend` true)
  (bind (_direction _alpha) (`Timeline|Timeline` :!label _label)
    (:`Update`
      (`KismetSystemLibrary.PrintString` "Open")
      (`SceneComponent.K2_SetRelativeRotation` (`self.DefaultSceneRoot`) (`KismetMathLibrary.RLerp` (`self.ActorRotation`) (`KismetMathLibrary.MakeRotator` _actorrotation_roll _actorrotation_pitch (+ _actorrotation_yaw 90.0)) _alpha) false false))))

(event `Closed`
  (set `self.bIsOpend` false)
  (goto _label :!via `Reverse`))

(fn `UserConstructionScript`
  (set `self.ActorRotation` (`self.K2_GetActorRotation`)))
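; BP_ThreeDoor is a puzzle door child Blueprint that unlocks when three inventory items are inserted in the correct order.
; OnUnlock moves the selected item into the first free slot and lights that slot's point light.
; Once full, it concatenates the three names and compares them to RequiredKeyName.
; A mismatch or empty-handed use returns items and resets the door, the latter also showing the locked message if locked.
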(event `self.ReceiveBeginPlay`
  (`parent.ReceiveBeginPlay`)
  (set `self.PointLights` (`|MakeArray` (`self.PointLight`) (`self.PointLight1`) (`self.PointLight2`))))

(fn `Light`
  (params (Index :type Integer))
  (`SceneComponent.SetVisibility` (`|GetArrayItem` (`self.PointLights`) Index) true false))

(fn `OnDoorClose`
  (`parent.OnDoorClose`)
  (`self.Closed`))

(fn `OnDoorOpen`
  (`parent.OnDoorOpen`)
  (`self.OpenDoor`))

(fn `OnUnlock`
  (params (RowName :type Name))
  (`parent.OnUnlock` RowName)
  (if (not (== (`|GetArrayItem` (`/Game/Blueprint/Character/BP_Player.Inventory` (`self.PlayerRef`)) (`/Game/Blueprint/Core/BP_Controller.CurrentSlotIndex` (`self.ControllerRef`))) "None"))
    (for (_array_element _array_index) (`self.RequiredNameThree`)
      (if (== _array_element "None")
        (`KismetArrayLibrary.Array_Set` (`self.RequiredNameThree`) _array_index (`|GetArrayItem` (`/Game/Blueprint/Character/BP_Player.Inventory` (`self.PlayerRef`)) (`/Game/Blueprint/Core/BP_Controller.CurrentSlotIndex` (`self.ControllerRef`))))
        (`self.Light` _array_index)
        (break)))
    (`KismetArrayLibrary.Array_Set` (`/Game/Blueprint/Character/BP_Player.Inventory` (`self.PlayerRef`)) (`/Game/Blueprint/Core/BP_Controller.CurrentSlotIndex` (`self.ControllerRef`)))
    (message `/Game/Blueprint/Interfacetable/BPI_OnInventoryUpdated.OnInventoryUpdated` (`self.HUDRef`))
    (if (not (`KismetArrayLibrary.Array_Contains` (`self.RequiredNameThree`)))
      (for _array_element_2 (`self.RequiredNameThree`)
        (bind _output_get (set `self.ComparisonName` (`KismetStringLibrary.Concat_StrStr` (`self.ComparisonName`) (`KismetStringLibrary.Conv_NameToString` _array_element_2)))))
      (if (== (`KismetStringLibrary.Conv_StringToName` _output_get) (`self.RequiredKeyName`))
        (set `self.bIsLocked` false)
        (else
          (for (_ _array_index_2) (`self.RequiredNameThree`) :!label _label
            (for (_array_element_3 _array_index_3) (`/Game/Blueprint/Character/BP_Player.Inventory` (`self.PlayerRef`))
              (if (== _array_element_3 "None")
                (`KismetArrayLibrary.Array_Set` (`/Game/Blueprint/Character/BP_Player.Inventory` (`self.PlayerRef`)) _array_index_3 (`|GetArrayItem` (`self.RequiredNameThree`) _array_index_2))
                (`SceneComponent.SetVisibility` (`self.PointLight`) false false)
                (`SceneComponent.SetVisibility` (`self.PointLight1`) false false)
                (`SceneComponent.SetVisibility` (`self.PointLight2`) false false)
                (break)))
            (message `/Game/Blueprint/Interfacetable/BPI_OnInventoryUpdated.OnInventoryUpdated` (`self.HUDRef`)))
          (set `self.RequiredNameThree` (`|MakeArray` "None" "None" "None" :!type "Name"))
          (set `self.ComparisonName` ""))))
    (else
      (`|ExecutionSequence`
        (:`then_0`
          (goto _label))
        (:`then_1`
          (if (`self.bIsLocked`)
            (`/Game/Blueprint/UI/WBP_UI_Main.LockDoorTextEvent` (`/Game/Blueprint/Core/BP_HUD.MainUiRef` (`self.HUDRef`)))))))))

(fn `UserConstructionScript`
  (`parent.UserConstructionScript`))
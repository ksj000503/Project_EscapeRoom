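; Password-locked drawer puzzle actor built on a parent door Blueprint, playing drawer open and close behavior on the door events.
; An unlock attempt brings up the HUD's password UI and binds an event to its check dispatcher.
; CheckPassword compares the entered password, as a Name, to the required key name, clearing the lock and calling the password UI again on a match, otherwise triggering the main UI's locked-door text.
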(event `CheckPassword`
  (params (Password :type String))
  (if (== (`KismetStringLibrary.Conv_StringToName` Password) (`self.RequiredKeyName`))
    (set `self.bIsLocked` false)
    (`/Game/Blueprint/Core/BP_HUD.PassWordUI` (`self.HUDRef`))
    (else
      (`/Game/Blueprint/UI/WBP_UI_Main.LockDoorTextEvent` (`/Game/Blueprint/Core/BP_HUD.MainUiRef` (`self.HUDRef`))))))

(fn `OnDoorClose`
  (`parent.OnDoorClose`)
  (`self.ClosedDrawer`))

(fn `OnDoorOpen`
  (`parent.OnDoorOpen`)
  (`self.OpenDrawer`))

(fn `OnUnlock`
  (params (RowName :type Name))
  (`parent.OnUnlock` "None")
  (`/Game/Blueprint/Core/BP_HUD.PassWordUI` (`self.HUDRef`))
  (add `/Game/Blueprint/UI/WBP_PasswordUI.OnCheck` (`/Game/Blueprint/Core/BP_HUD.PasswordUIRef` (`self.HUDRef`)) (`|CreateDelegate` :!event `CheckPassword`)))

(fn `UserConstructionScript`
  (`parent.UserConstructionScript`))
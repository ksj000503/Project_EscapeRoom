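; BP_Door_Slider is a sliding puzzle door, built on a parent door class, that can be unlocked with a key from the player's inventory.
; Open and close overrides call the parent logic, then trigger the slider motion.
; Unlocking compares the selected inventory slot to the required key name: a match clears the lock and empties that slot, while a mismatch shows locked-door text on the HUD.
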(fn `OnDoorClose`
  (`parent.OnDoorClose`)
  (`self.ClosedSlider`))

(fn `OnDoorOpen`
  (`parent.OnDoorOpen`)
  (`self.OpenSlider`))

(fn `OnUnlock`
  (params (RowName :type Name))
  (`parent.OnUnlock` "None")
  (if (== (`|GetArrayItem` (`/Game/Blueprint/Character/BP_Player.Inventory` (`self.PlayerRef`)) (`/Game/Blueprint/Core/BP_Controller.CurrentSlotIndex` (`self.ControllerRef`))) (`self.RequiredKeyName`))
    (set `self.bIsLocked` false)
    (`KismetArrayLibrary.Array_Set` (`/Game/Blueprint/Character/BP_Player.Inventory` (`self.PlayerRef`)) (`/Game/Blueprint/Core/BP_Controller.CurrentSlotIndex` (`self.ControllerRef`)))
    (else
      (`/Game/Blueprint/UI/WBP_UI_Main.LockDoorTextEvent` (`/Game/Blueprint/Core/BP_HUD.MainUiRef` (`self.HUDRef`))))))

(fn `UserConstructionScript`
  (`parent.UserConstructionScript`))
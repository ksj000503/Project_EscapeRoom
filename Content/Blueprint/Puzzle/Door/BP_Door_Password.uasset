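; Password-locked puzzle door, extending a parent door that provides the lock state and open/close hooks.
; Unlocking calls the HUD's password UI and binds an event to its check callback, passing no key row to the parent.
; CheckPassword compares the entry to RequiredKeyName, clearing the lock and calling the password UI again on a match, or showing locked-door text otherwise.
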(event `CheckPassword`
  (params (PasswordValue :type String))
  (if (== (`KismetStringLibrary.Conv_StringToName` PasswordValue) (`self.RequiredKeyName`))
    (set `self.bIsLocked` false)
    (`/Game/Blueprint/Core/BP_HUD.PassWordUI` (`self.HUDRef`))
    (else
      (`/Game/Blueprint/UI/WBP_UI_Main.LockDoorTextEvent` (`/Game/Blueprint/Core/BP_HUD.MainUiRef` (`self.HUDRef`))))))

(fn `OnDoorClose`
  (`parent.OnDoorClose`)
  (`self.Closed`))

(fn `OnDoorOpen`
  (`parent.OnDoorOpen`)
  (`self.OpenDoor`))

(fn `OnUnlock`
  (params (RowName :type Name))
  (`parent.OnUnlock` "None")
  (`/Game/Blueprint/Core/BP_HUD.PassWordUI` (`self.HUDRef`))
  (add `/Game/Blueprint/UI/WBP_PasswordUI.OnCheck` (`/Game/Blueprint/Core/BP_HUD.PasswordUIRef` (`self.HUDRef`)) (`|CreateDelegate` :!event `CheckPassword`)))

(fn `UserConstructionScript`
  (`parent.UserConstructionScript`))
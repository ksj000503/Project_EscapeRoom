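; Door Blueprint for puzzles that unlocks with a named key item from the player's inventory.
; Unlocking compares the given row name to the required key, clears the locked flag and overwrites the current inventory slot with an empty entry, consuming the key.
; Open and close overrides call the parent logic, then this door's own open and close routines.
; Despite the asset's name, its overlap event is an unused stub.
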(fn `OnDoorClose`
  (`parent.OnDoorClose`)
  (`self.Closed`))

(fn `OnDoorOpen`
  (`parent.OnDoorOpen`)
  (`self.OpenDoor`))

(fn `OnUnlock`
  (params (RowName :type Name))
  (if (== RowName (`self.RequiredKeyName`))
    (set `self.bIsLocked` false)
    (`KismetArrayLibrary.Array_Set` (`/Game/Blueprint/Character/BP_Player.Inventory` (`self.PlayerRef`)) (`/Game/Blueprint/Core/BP_Controller.CurrentSlotIndex` (`self.ControllerRef`)))))

(fn `UserConstructionScript`
  (`parent.UserConstructionScript`))
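; BP_Door_Drawer is a lockable drawer variant of a parent door Blueprint, used among the puzzle doors.
; Its open and close overrides call the parent logic, then OpenDrawer or ClosedDrawer.
; On unlock, it compares the player's selected inventory slot to RequiredKeyName; a match clears the lock and resets that slot, otherwise the HUD fires its locked-door text event.
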(fn `OnDoorClose`
  (`parent.OnDoorClose`)
  (`self.ClosedDrawer`))

(fn `OnDoorOpen`
  (`parent.OnDoorOpen`)
  (`self.OpenDrawer`))

(fn `OnUnlock`
  (params (RowName :type Name))
  (`parent.OnUnlock` "None")
  (if (== (`|GetArrayItem` (`/Game/Blueprint/Character/BP_Player.Inventory` (`self.PlayerRef`)) (`/Game/Blueprint/Core/BP_Controller.CurrentSlotIndex` (`self.ControllerRef`))) (`self.RequiredKeyName`))
    (set `self.bIsLocked` false)
    (`KismetArrayLibrary.Array_Set` (`/Game/Blueprint/Character/BP_Player.Inventory` (`self.PlayerRef`)) (`/Game/Blueprint/Core/BP_Controller.CurrentSlotIndex` (`self.ControllerRef`)))
    (else
      (`/Game/Blueprint/UI/WBP_UI_Main.LockDoorTextEvent` (`/Game/Blueprint/Core/BP_HUD.MainUiRef` (`self.HUDRef`))))))

(fn `UserConstructionScript`
  (`parent.UserConstructionScript`))
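; BP_Door_Base is a base puzzle door configured by a DT_DoorDatas row supplying mesh, lock state, required key, door type and open amount.
; LockDoorOpen calls OnUnlock when locked, otherwise OnDoorOpen or OnDoorClose, all empty here.
; Separate timeline events move the root for hinged doors (yaw), sliders (X) and drawers (Y), reversing to close.
; The construction script applies the mesh, while BeginPlay caches player references and the starting transform.
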(event `self.ReceiveBeginPlay`
  (`self.Ref`)
  (`self.DoorInit`)
  (set `self.ActorRotation` (`self.K2_GetActorRotation`))
  (set `self.ActorLocation` (`self.K2_GetActorLocation`)))

(event `/Game/Blueprint/Interfacetable/BPI_LockDoorOpen.LockDoorOpen`
  (params (RowName :type Name))
  (if (`self.bIsLocked`)
    (`self.OnUnlock` "None")
    (elif (not (`self.bIsOpend`))
      (`self.OnDoorOpen`)
      (else
        (`self.OnDoorClose`)))))

(event `OpenDoor`
  (bind (_actorrotation_roll _actorrotation_pitch _actorrotation_yaw) (`KismetMathLibrary.BreakRotator` (`self.ActorRotation`)))
  (set `self.bIsOpend` true)
  (bind (_direction _alpha) (`Timeline|OpenDoorTimeLine` :!label _label)
    (:`Update`
      (`SceneComponent.K2_SetRelativeRotation` (`self.DefaultSceneRoot`) (`KismetMathLibrary.RLerp` (`self.ActorRotation`) (`KismetMathLibrary.MakeRotator` _actorrotation_roll _actorrotation_pitch (+ _actorrotation_yaw (break `/Game/Blueprint/Datas/Struct/ST_DoorOpen` (`.OpenValue_9_B29E50CF496636A59DAF7BB2C5435B72` (break `/Game/Blueprint/Datas/Struct/ST_DoorData` (`self.Out Row`)))))) _alpha) false false))))

(event `Closed`
  (set `self.bIsOpend` false)
  (goto _label :!via `Reverse`))

(event `OpenSlider`
  (bind (_actorlocation_x _actorlocation_y _actorlocation_z) (`KismetMathLibrary.BreakVector` (`self.ActorLocation`)))
  (set `self.bIsOpend` true)
  (bind (_direction _alpha) (`Timeline|Timeline` :!label _label_2)
    (:`Update`
      (`SceneComponent.K2_SetRelativeLocation` (`self.DefaultSceneRoot`) (`KismetMathLibrary.VLerp` (`self.ActorLocation`) (`KismetMathLibrary.MakeVector` (- _actorlocation_x (break `/Game/Blueprint/Datas/Struct/ST_DoorOpen` (`.OpenValue_9_B29E50CF496636A59DAF7BB2C5435B72` (break `/Game/Blueprint/Datas/Struct/ST_DoorData` (`self.Out Row`))))) _actorlocation_y _actorlocation_z) _alpha) false false))))

(event `ClosedSlider`
  (set `self.bIsOpend` false)
  (goto _label_2 :!via `Reverse`))

(event `OpenDrawer`
  (bind (_actorlocation_x _actorlocation_y _actorlocation_z) (`KismetMathLibrary.BreakVector` (`self.ActorLocation`)))
  (set `self.bIsOpend` true)
  (bind (_direction _alpha) (`Timeline|DrawerOpen` :!label _label_3)
    (:`Update`
      (`SceneComponent.K2_SetRelativeLocation` (`self.DefaultSceneRoot`) (`KismetMathLibrary.VLerp` (`self.ActorLocation`) (`KismetMathLibrary.MakeVector` _actorlocation_x (+ _actorlocation_y (break `/Game/Blueprint/Datas/Struct/ST_DoorOpen` (`.OpenValue_9_B29E50CF496636A59DAF7BB2C5435B72` (break `/Game/Blueprint/Datas/Struct/ST_DoorData` (`self.Out Row`))))) _actorlocation_z) _alpha) false false))))

(event `ClosedDrawer`
  (set `self.bIsOpend` false)
  (goto _label_3 :!via `Reverse`))

(fn `DoorInit`
  (bind _rowname (`self.RowName`))
  (bind (_out_row_locked _out_row_membervar_1 _out_row_requiredkeyname _out_row_openvalue _out_row_doortype _out_row_locktype) (break `/Game/Blueprint/Datas/Struct/ST_DoorData` (`self.Out Row`)))
  (bind _returnvalue (`|GetDataTableRow` "/Game/Blueprint/Datas/DataTable/DT_DoorDatas.DT_DoorDatas" _rowname)
    (:`then`
      (set `self.Out Row` _returnvalue)
      (`StaticMeshComponent.SetStaticMesh` (`self.StaticMesh`) _out_row_membervar_1)
      (set `self.bIsLocked` _out_row_locked)
      (set `self.RequiredKeyName` _out_row_requiredkeyname)
      (set `self.DoorsType` _out_row_doortype)
      (set `self.Out Row Lock Type` _out_row_locktype))
    (:`RowNotFound`
      (`KismetSystemLibrary.PrintString` (`KismetStringLibrary.Conv_NameToString` _rowname)))))

(fn `LockDoor`
  (returns (Looked :type Boolean))
  (return (`self.bIsLocked`)))

(fn `OnDoorClose`)

(fn `OnDoorOpen`)

(fn `OnUnlock`
  (params (RowName :type Name)))

(fn `Ref`
  (bind _asbp_controller (cast `/Game/Blueprint/Core/BP_Controller` (`GameplayStatics.GetPlayerController` 0)))
  (set `self.ControllerRef` _asbp_controller)
  (bind _asbp_hud (cast `/Game/Blueprint/Core/BP_HUD` (`PlayerController.GetHUD` (`GameplayStatics.GetPlayerController` 0))))
  (set `self.HUDRef` _asbp_hud)
  (bind _asbp_player (cast `/Game/Blueprint/Character/BP_Player` (`GameplayStatics.GetPlayerCharacter` 0)))
  (set `self.PlayerRef` _asbp_player))

(fn `UserConstructionScript`
  (bind _rowname (`self.RowName`))
  (bind (_out_row_locked _out_row_membervar_1) (break `/Game/Blueprint/Datas/Struct/ST_DoorData` (`self.Out Row`)))
  (bind _returnvalue (`|GetDataTableRow` "/Game/Blueprint/Datas/DataTable/DT_DoorDatas.DT_DoorDatas" _rowname)
    (:`then`
      (set `self.Out Row` _returnvalue)
      (`StaticMeshComponent.SetStaticMesh` (`self.StaticMesh`) _out_row_membervar_1))
    (:`RowNotFound`
      (`KismetSystemLibrary.PrintString` (`KismetStringLibrary.Conv_NameToString` _rowname)))))
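; BP_Lock_Base is the base Blueprint for puzzle locks, exposing a lock state for doors.
; Its construction script looks up RowName in DT_LockData and applies that row's 3D mesh to the static mesh component.
; On BeginPlay it caches the BP_Player reference and calls LockDoorMessage, whose body is not in this graph.
; The LockDoor function returns the IsLock flag.
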(event `self.ReceiveBeginPlay`
  (bind _asbp_player (cast `/Game/Blueprint/Character/BP_Player` (`GameplayStatics.GetPlayerCharacter` 0)))
  (set `self.As BP Player` _asbp_player)
  (message `/Game/Blueprint/Interfacetable/BPI_LockDoor.LockDoor` self))

(fn `LockDoor`
  (returns (Looked :type Boolean))
  (return (`self.bIsLock`)))

(fn `UserConstructionScript`
  (bind _returnvalue (`|GetDataTableRow` "/Game/Blueprint/Datas/DataTable/DT_LockData.DT_LockData" (`self.RowName`))
    (:`then`
      (bind _output_get (set `self.Out Row` _returnvalue))
      (`StaticMeshComponent.SetStaticMesh` (`self.StaticMesh`) (`.3DMesh_6_527042E1446982F6530F94A61683AA3E` (break `/Game/Blueprint/Datas/Struct/ST_LockData` _output_get))))))
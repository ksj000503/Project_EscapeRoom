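; Base puzzle door actor that opens and closes as one of three types: hinged door, slider or drawer.
; The construction script reads mesh, lock state, key name and type from a DT_DoorDatas row.
; DoorTypeOpen and DoorTypeClosed dispatch to timelines that lerp root yaw, X or Y by the row's open value, reversing to close.
; BeginPlay binds to BP_chess's OnOpenDoor, but that handler is empty; LockDoor only reports IsLocked.
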(event `self.ReceiveBeginPlay`
  (set `self.ActorRotation` (`self.K2_GetActorRotation`))
  (set `self.ActorLocation` (`self.K2_GetActorLocation`))
  (bind _returnvalue (`GameplayStatics.GetActorOfClass` "/Game/Blueprint/Puzzle/BP_chess.BP_chess_C"))
  (bind _output_get (set `self.ChessRef` _returnvalue))
  (add `/Game/Blueprint/Puzzle/BP_chess.OnOpenDoor` _output_get (delegate `CustomEvent`)))

(event `CustomEvent`)

(event `DoorTypeOpen`
  (if (`|EnumEquality` (`self.DoorsType`) "NewEnumerator0")
    (`self.OpenDoor`)
    (elif (`|EnumEquality` (`self.DoorsType`) "NewEnumerator1")
      (`self.OpenSlider`)
      (elif (`|EnumEquality` (`self.DoorsType`) "NewEnumerator2")
        (`self.OpenDrawer`)))))

(event `DoorTypeClosed`
  (if (`|EnumEquality` (`self.DoorsType`) "NewEnumerator0")
    (`self.Closed`)
    (elif (`|EnumEquality` (`self.DoorsType`) "NewEnumerator1")
      (`self.ClosedSlider`)
      (elif (`|EnumEquality` (`self.DoorsType`) "NewEnumerator2")
        (`self.ClosedDrawer`)))))

(event `OpenDoor`
  (bind (_actorrotation_roll _actorrotation_pitch _actorrotation_yaw) (`KismetMathLibrary.BreakRotator` (`self.ActorRotation`)))
  (set `self.bIsOpend` true)
  (bind (_direction _alpha) (`Timeline|OpenDoorTimeLine` :!label _label)
    (:`Update`
      (`SceneComponent.K2_SetRelativeRotation` (`self.DefaultSceneRoot`) (`KismetMathLibrary.RLerp` (`self.ActorRotation`) (`KismetMathLibrary.MakeRotator` _actorrotation_roll _actorrotation_pitch (+ _actorrotation_yaw (break `/Game/Blueprint/Datas/Struct/ST_DoorOpen` (`.OpenValue_9_B29E50CF496636A59DAF7BB2C5435B72` (break `/Game/Blueprint/Datas/Struct/ST_DoorData` (`self.Out Row`)))))) _alpha) false false))))

(event `Closed`
  (set `self.bIsOpend` false)
  (goto _label :!via `Reverse`))

(event `OpenSlider`
  (bind (_actorlocation_x _actorlocation_y _actorlocation_z) (`KismetMathLibrary.BreakVector` (`self.ActorLocation`)))
  (set `self.bIsOpend` true)
  (bind (_direction _alpha) (`Timeline|Timeline` :!label _label_2)
    (:`Update`
      (`SceneComponent.K2_SetRelativeLocation` (`self.DefaultSceneRoot`) (`KismetMathLibrary.VLerp` (`self.ActorLocation`) (`KismetMathLibrary.MakeVector` (- _actorlocation_x (break `/Game/Blueprint/Datas/Struct/ST_DoorOpen` (`.OpenValue_9_B29E50CF496636A59DAF7BB2C5435B72` (break `/Game/Blueprint/Datas/Struct/ST_DoorData` (`self.Out Row`))))) _actorlocation_y _actorlocation_z) _alpha) false false))))

(event `ClosedSlider`
  (set `self.bIsOpend` false)
  (goto _label_2 :!via `Reverse`))

(event `OpenDrawer`
  (bind (_actorlocation_x _actorlocation_y _actorlocation_z) (`KismetMathLibrary.BreakVector` (`self.ActorLocation`)))
  (set `self.bIsOpend` true)
  (bind (_direction _alpha) (`Timeline|DrawerOpen` :!label _label_3)
    (:`Update`
      (`SceneComponent.K2_SetRelativeLocation` (`self.DefaultSceneRoot`) (`KismetMathLibrary.VLerp` (`self.ActorLocation`) (`KismetMathLibrary.MakeVector` _actorlocation_x (+ _actorlocation_y (break `/Game/Blueprint/Datas/Struct/ST_DoorOpen` (`.OpenValue_9_B29E50CF496636A59DAF7BB2C5435B72` (break `/Game/Blueprint/Datas/Struct/ST_DoorData` (`self.Out Row`))))) _actorlocation_z) _alpha) false false))))

(event `ClosedDrawer`
  (set `self.bIsOpend` false)
  (goto _label_3 :!via `Reverse`))

(fn `LockDoor`
  (returns (Looked :type Boolean))
  (return (`self.bIsLocked`)))

(fn `UserConstructionScript`
  (bind (_out_row_locked _out_row_membervar_1 _out_row_requiredkeyname _out_row_openvalue _out_row_doortype) (break `/Game/Blueprint/Datas/Struct/ST_DoorData` (`self.Out Row`)))
  (bind _returnvalue (`|GetDataTableRow` "/Game/Blueprint/Datas/DataTable/DT_DoorDatas.DT_DoorDatas" (`self.RowName`))
    (:`then`
      (set `self.Out Row` _returnvalue)
      (`StaticMeshComponent.SetStaticMesh` (`self.StaticMesh`) _out_row_membervar_1)
      (set `self.bIsLocked` _out_row_locked)
      (set `self.RequiredKeyName` _out_row_requiredkeyname)
      (set `self.DoorsType` _out_row_doortype))))